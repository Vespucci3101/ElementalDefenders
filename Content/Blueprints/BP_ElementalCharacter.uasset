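; Player character for a multiplayer elemental game: creates HUD widgets, fires camera-aimed class projectiles, triggers zones and casts two GameInstance-selected abilities.
; Auto-spawn abilities spawn through server events; others spawn a client preview that can be cancelled or click-confirmed into a damaging server spawn.
; Movement dispatches on class display name: traced ground targeting with zoomed-out camera, or thrower transforms applied through GameMode lists keyed by client name.
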(event `self.ReceiveBeginPlay`
  (bind _returnvalue (`|CreateWidget` "/Game/UI/WBP_PlayerHealthAndAbilities.WBP_PlayerHealthAndAbilities_C"))
  (`UserWidget.AddToViewport` _returnvalue 0)
  (set `self.HealthAndAbilitiesWBP` _returnvalue)
  (bind _returnvalue_2 (`|CreateWidget` "/Game/UI/WBP_Crosshair.WBP_Crosshair_C"))
  (`UserWidget.AddToViewport` _returnvalue_2 0))

(event `self.ReceiveTick`
  (params (DeltaSeconds :type "Float (single-precision)"))
  (bind _health (`self.Health`))
  (bind _followfirstability (`self.FollowFirstAbility`))
  (if (`self.IsAttacking`)
    (set `self.IsAttacking` false)
    (`/Game/UI/WBP_PlayerHealthAndAbilities.Update Health` (`self.HealthAndAbilitiesWBP`) (`HealthComponent.health` _health) (`HealthComponent.maxHealth` _health))
    (if (or (`self.FollowSecondAbility`) _followfirstability)
      (`self.AbilitiesMovement` _followfirstability))))

(event `Server Update Ability transform`
  (params (Transform :type "Transform Structure") (ClientName :type String) (IsServer :type Boolean) (IsFirstAbility :type Boolean))
  (`self.ServerAbilityUpdateMovements` Transform ClientName IsServer IsFirstAbility))

(event `InputAction|Interact`
  (params (Key :type "Key Structure"))
  (:`Pressed`
    (if (`self.CanInteractWithZone`)
      (bind _asbp_unactivated_zone (cast `/Game/Blueprints/BP_UnactivatedZone` (`self.InteractableZone`)))
      (`/Game/Blueprints/BP_UnactivatedZone.Trigger Zone` _asbp_unactivated_zone))))

(event `InputAction|CancelAbility`
  (params (Key :type "Key Structure"))
  (:`Pressed`
    (if (`self.IsFirstAbilityCast`)
      (`self.CancelFirstAbility`)
      (else
        (`self.CancelSecondAbility`)))))

(event `InputAction|Fire`
  (params (Key :type "Key Structure"))
  (:`Pressed`
    (if (`self.CanFireProjectile`)
      (set `self.IsAttacking` true)
      (`self.SetProjectileSpwanPointRotation`)
      (bind _asbp_elemental_game_instance (cast `/Game/Blueprints/BP_ElementalGameInstance` (`GameplayStatics.GetGameInstance`)))
      (`self.SpawnProjectile` (`/Game/Blueprints/BP_ElementalGameInstance.CharacterClass` _asbp_elemental_game_instance))
      (elif (`self.IsFirstAbilityCast`)
        (`self.First Ability Spawn On Click`)
        (else
          (`self.SecondAbilitySpawnOnClick`))))))

(event `SpawnProjectile`
  (params (`Character Class` :type String))
  (bind _returnvalue (`|SpawnActorFromClass` "/Game/Blueprints/Abilities/BP_Projectile.BP_Projectile_C" (`SceneComponent.K2_GetComponentToWorld` (`self.ProjectileSpawnPoint`)) "Undefined" "OverrideRootScale" null null))
  (`self.SetOwner` _returnvalue self)
  (`/Game/Blueprints/Abilities/BP_Projectile.Set Projectile Class` _returnvalue `Character Class`))

(event `SetProjectileSpwanPointRotation`
  (bind _returnvalue (`self.K2_GetActorLocation`))
  (bind _cameracomponent (`self.CameraComponent`))
  (bind _projectilespawnpoint (`self.ProjectileSpawnPoint`))
  (bind _returnvalue_2 (`SceneComponent.K2_GetComponentLocation` _cameracomponent))
  (bind _returnvalue_3 (+ (* (`SceneComponent.GetForwardVector` _cameracomponent) 5000.0) _returnvalue_2))
  (bind (_outhit _returnvalue_4) (`KismetSystemLibrary.LineTraceSingle` _returnvalue_2 _returnvalue_3 "TraceTypeQuery1"))
  (if _returnvalue_4
    (`SceneComponent.K2_SetWorldRotation` _projectilespawnpoint (`KismetMathLibrary.Conv_VectorToRotator` (- (`.Location` (`GameplayStatics.BreakHitResult` _outhit)) _returnvalue)) false false)
    (else
      (`SceneComponent.K2_SetWorldRotation` _projectilespawnpoint (`KismetMathLibrary.Conv_VectorToRotator` (- _returnvalue_3 _returnvalue)) false false))))

(event `InputAction|FirstAbility`
  (params (Key :type "Key Structure"))
  (bind _visor_transform (`self.GetVisorTransfrom`))
  (bind _isalreadyincast (`self.IsAlreadyInCast`))
  (:`Pressed`
    (bind _asbp_elemental_game_instance (cast `/Game/Blueprints/BP_ElementalGameInstance` (`GameplayStatics.GetGameInstance`)))
    (`self.SetProjectileSpwanPointRotation`)
    (bind _isfirstabilityautospawn (`/Game/Blueprints/BP_ElementalGameInstance.IsFirstAbilityAutoSpawn` _asbp_elemental_game_instance))
    (if _isfirstabilityautospawn
      (bind _firstabilityclass (`/Game/Blueprints/BP_ElementalGameInstance.FirstAbilityClass` _asbp_elemental_game_instance))
      (`self.Server Spawn First Ability` _firstabilityclass _visor_transform _isfirstabilityautospawn (`KismetSystemLibrary.IsServer`) _isalreadyincast self)
      (else
        (`self.Client Spawn First Ability` _firstabilityclass _visor_transform _isalreadyincast)))
    (set `self.CanFireProjectile` false)
    (set `self.IsAlreadyInCast` true)
    (set `self.FollowFirstAbility` true)
    (set `self.IsFirstAbilityCast` true)))

(event `Server Spawn First Ability`
  (params (`Actor Class` :type "Actor Class Reference") (Transform :type "Transform Structure") (IsAutoSpawn :type Boolean) (IsServer :type Boolean) (IsAlreadyInCast :type Boolean) (Owner :type "Actor Object Reference"))
  (if (not IsAlreadyInCast)
    (bind _returnvalue (`|SpawnActorFromClass` `Actor Class` Transform "Undefined" "OverrideRootScale" null null))
    (`self.SetOwner` _returnvalue Owner)
    (`self.First Ability Trigger Damage` _returnvalue)
    (if (or IsAutoSpawn IsServer)
      (bind _asbp_elemental_defender_game_mode_base (cast `/Game/Blueprints/BP_ElementalDefenderGameModeBase` (`GameplayStatics.GetGameMode`)))
      (`/Game/Blueprints/BP_ElementalDefenderGameModeBase.UpdateAbilityLists` _asbp_elemental_defender_game_mode_base (`KismetSystemLibrary.GetDisplayName` Owner) _returnvalue true))))

(event `Client Spawn First Ability`
  (params (`Actor Class` :type "Actor Class Reference") (Transform :type "Transform Structure") (IsAlreadyInCast :type Boolean))
  (if (not IsAlreadyInCast)
    (bind _returnvalue (`|SpawnActorFromClass` `Actor Class` Transform "Undefined" "OverrideRootScale" null null))
    (`self.SetOwner` _returnvalue self)
    (set `self.FirstAbilityRef` _returnvalue)))

(event `InputAction|SecondAbility`
  (params (Key :type "Key Structure"))
  (bind _visor_transform (`self.GetVisorTransfrom`))
  (bind _isalreadyincast (`self.IsAlreadyInCast`))
  (:`Pressed`
    (bind _asbp_elemental_game_instance (cast `/Game/Blueprints/BP_ElementalGameInstance` (`GameplayStatics.GetGameInstance`)))
    (`self.SetProjectileSpwanPointRotation`)
    (bind _issecondabilityautospawn (`/Game/Blueprints/BP_ElementalGameInstance.IsSecondAbilityAutoSpawn` _asbp_elemental_game_instance))
    (if _issecondabilityautospawn
      (bind _secondabilityclass (`/Game/Blueprints/BP_ElementalGameInstance.SecondAbilityClass` _asbp_elemental_game_instance))
      (`self.Server Spawn Second Ability` _secondabilityclass _visor_transform _issecondabilityautospawn (`KismetSystemLibrary.IsServer`) _isalreadyincast self)
      (else
        (`self.Client Spawn Second Ability` _secondabilityclass _visor_transform _isalreadyincast)))
    (set `self.CanFireProjectile` false)
    (set `self.IsAlreadyInCast` true)
    (set `self.FollowSecondAbility` true)
    (set `self.IsFirstAbilityCast` false)))

(event `Server Spawn Second Ability`
  (params (`Actor Class` :type "Actor Class Reference") (transform :type "Transform Structure") (IsAutoSpawn :type Boolean) (IsServer :type Boolean) (AlreadyInCast :type Boolean) (Owner :type "Actor Object Reference"))
  (if (not AlreadyInCast)
    (bind _returnvalue (`|SpawnActorFromClass` `Actor Class` transform "Undefined" "OverrideRootScale" null null))
    (`self.SetOwner` _returnvalue Owner)
    (`self.Second Ability Trigger Damage` _returnvalue)
    (if (or IsAutoSpawn IsServer)
      (bind _asbp_elemental_defender_game_mode_base (cast `/Game/Blueprints/BP_ElementalDefenderGameModeBase` (`GameplayStatics.GetGameMode`)))
      (`/Game/Blueprints/BP_ElementalDefenderGameModeBase.UpdateAbilityLists` _asbp_elemental_defender_game_mode_base (`KismetSystemLibrary.GetDisplayName` Owner) _returnvalue false))))

(event `Client Spawn Second Ability`
  (params (`Actor Class` :type "Actor Class Reference") (Transform :type "Transform Structure") (IsAlreadyInCast :type Boolean))
  (if (not IsAlreadyInCast)
    (bind _returnvalue (`|SpawnActorFromClass` `Actor Class` Transform "Undefined" "OverrideRootScale" null null))
    (`self.SetOwner` _returnvalue self)
    (set `self.SecondAbilityRef` _returnvalue)))

(fn `AbilitiesMovement`
  (params (IsFollowingFirstAbility :type Boolean))
  (locals (`Ability Name` :type String) (`Ability Ref` :type "Actor Object Reference"))
  (if IsFollowingFirstAbility
    (bind _asbp_elemental_game_instance (cast `/Game/Blueprints/BP_ElementalGameInstance` (`GameplayStatics.GetGameInstance`)))
    (set `local.Ability Name` (`KismetSystemLibrary.GetClassDisplayName` (`/Game/Blueprints/BP_ElementalGameInstance.FirstAbilityClass` _asbp_elemental_game_instance)))
    (switch `string` (`local.Ability Name`)
      (:`BP_FlameThrowerAbility_C`
        (`self.Flamethrower Movement`))
      (:`BP_WaterDropletsAbility_C`
        (`self.Water Droplets Movement` (`self.FirstAbilityRef`)))
      (:`BP_IceThrowerAbility_C`
        (`self.IceThrower Movement`)))
    (else
      (bind _asbp_elemental_game_instance_2 (cast `/Game/Blueprints/BP_ElementalGameInstance` (`GameplayStatics.GetGameInstance`)))
      (set `local.Ability Name` (`KismetSystemLibrary.GetClassDisplayName` (`/Game/Blueprints/BP_ElementalGameInstance.SecondAbilityClass` _asbp_elemental_game_instance_2)))
      (switch `string` (`local.Ability Name`)
        (:`BP_MeteorAbility_C`
          (`self.Meteor Movement` (`self.SecondAbilityRef`)))
        (:`BP_TsunamiAbility_C`
          (`self.TsunamiAbilityMovement` (`self.SecondAbilityRef`)))
        (:`BP_BlizzardAbility_C`
          (`self.Blizzard Ability Movement` (`self.SecondAbilityRef`)))))))

(fn `AbilityCancelEvents`
  (params (`Ability Class` :type "Actor Class Reference"))
  (switch `string` (`KismetSystemLibrary.GetClassDisplayName` `Ability Class`)
    (:`BP_WaterDropletsAbility_C`
      (bind _asbp_water_droplets_ability (cast `/Game/Blueprints/Abilities/BP_WaterDropletsAbility` (`self.FirstAbilityRef`)))
      (`/Game/Blueprints/Abilities/BP_WaterDropletsAbility.Cancel Ability` _asbp_water_droplets_ability))
    (:`BP_BlizzardAbility_C`
      (bind _asbp_blizzard_ability (cast `/Game/Blueprints/Abilities/BP_BlizzardAbility` (`self.SecondAbilityRef`)))
      (`/Game/Blueprints/Abilities/BP_BlizzardAbility.Cancel Ability` _asbp_blizzard_ability))
    (:`BP_TsunamiAbility_C`
      (bind _asbp_tsunami_ability (cast `/Game/Blueprints/Abilities/BP_TsunamiAbility` (`self.SecondAbilityRef`)))
      (`/Game/Blueprints/Abilities/BP_TsunamiAbility.Cancel Ability` _asbp_tsunami_ability))
    (:`BP_MeteorAbility_C`
      (bind _asbp_meteor_ability (cast `/Game/Blueprints/Abilities/BP_MeteorAbility` (`self.SecondAbilityRef`)))
      (`/Game/Blueprints/Abilities/BP_MeteorAbility.Cancel Ability` _asbp_meteor_ability))))

(fn `Blizzard Ability Movement`
  (params (`Ability Ref` :type "Actor Object Reference"))
  (bind _cameracomponent (`self.CameraComponent`))
  (bind _returnvalue (`SceneComponent.K2_GetComponentLocation` _cameracomponent))
  (`self.ZoomOutCameraView`)
  (`/Engine/EditorBlueprintResources/StandardMacros.IsValid` `Ability Ref`
    (:`Is Valid`
      (`self.SetProjectileSpwanPointRotation`)
      (bind (_outhit _returnvalue_2) (`KismetSystemLibrary.LineTraceSingle` _returnvalue (+ (* (`SceneComponent.GetForwardVector` _cameracomponent) 3000.0) _returnvalue) "TraceTypeQuery1"))
      (if _returnvalue_2
        (bind _output_get (set `self.Spawn Transform` (`KismetMathLibrary.MakeTransform` (`.Location` (`GameplayStatics.BreakHitResult` _outhit)) (`SceneComponent.K2_GetComponentRotation` (`self.ProjectileSpawnPoint`)))))
        (`self.K2_SetActorTransform` `Ability Ref` _output_get false false)))))

(fn `CancelFirstAbility`
  (bind _asbp_elemental_game_instance (cast `/Game/Blueprints/BP_ElementalGameInstance` (`GameplayStatics.GetGameInstance`)))
  (if (and (`self.IsAlreadyInCast`) (not (`/Game/Blueprints/BP_ElementalGameInstance.IsFirstAbilityAutoSpawn` _asbp_elemental_game_instance)))
    (`self.AbilityCancelEvents` (`/Game/Blueprints/BP_ElementalGameInstance.FirstAbilityClass` _asbp_elemental_game_instance))
    (`self.ZoomInCameraView`)
    (set `self.FollowFirstAbility` false)
    (set `self.CanFireProjectile` true)
    (set `self.IsAlreadyInCast` false)))

(fn `CancelSecondAbility`
  (bind _asbp_elemental_game_instance (cast `/Game/Blueprints/BP_ElementalGameInstance` (`GameplayStatics.GetGameInstance`)))
  (if (and (`self.IsAlreadyInCast`) (not (`/Game/Blueprints/BP_ElementalGameInstance.IsSecondAbilityAutoSpawn` _asbp_elemental_game_instance)))
    (`self.AbilityCancelEvents` (`/Game/Blueprints/BP_ElementalGameInstance.SecondAbilityClass` _asbp_elemental_game_instance))
    (`self.ZoomInCameraView`)
    (set `self.FollowSecondAbility` false)
    (set `self.CanFireProjectile` true)
    (set `self.IsAlreadyInCast` false)))

(fn `First Ability Spawn On Click`
  (bind _firstabilityref (`self.FirstAbilityRef`))
  (bind _asbp_elemental_game_instance (cast `/Game/Blueprints/BP_ElementalGameInstance` (`GameplayStatics.GetGameInstance`)))
  (bind _isfirstabilityautospawn (`/Game/Blueprints/BP_ElementalGameInstance.IsFirstAbilityAutoSpawn` _asbp_elemental_game_instance))
  (if (not _isfirstabilityautospawn)
    (bind _output_get (set `self.FirstAbilityTransform` (`self.GetTransform` _firstabilityref)))
    (`self.K2_DestroyActor` _firstabilityref)
    (set `self.FollowFirstAbility` false)
    (set `self.CanFireProjectile` true)
    (set `self.IsAlreadyInCast` false)
    (set `self.IsFirstAbilityCast` false)
    (`self.Server Spawn First Ability` (`/Game/Blueprints/BP_ElementalGameInstance.FirstAbilityClass` _asbp_elemental_game_instance) _output_get _isfirstabilityautospawn (`KismetSystemLibrary.IsServer`) (`self.IsAlreadyInCast`) (`Controller.K2_GetPawn` (`GameplayStatics.GetPlayerController` 0)))
    (`self.ZoomInCameraView`)))

(fn `First Ability Trigger Damage`
  (params (`Ability Ref` :type "Actor Object Reference"))
  (bind _asbp_elemental_game_instance (cast `/Game/Blueprints/BP_ElementalGameInstance` (`GameplayStatics.GetGameInstance`)))
  (switch `string` (`KismetSystemLibrary.GetClassDisplayName` (`/Game/Blueprints/BP_ElementalGameInstance.FirstAbilityClass` _asbp_elemental_game_instance))
    (:`BP_WaterDropletsAbility_C`
      (bind _asbp_water_droplets_ability (cast `/Game/Blueprints/Abilities/BP_WaterDropletsAbility` `Ability Ref`))
      (`/Game/Blueprints/Abilities/BP_WaterDropletsAbility.Trigger Damage` _asbp_water_droplets_ability))))

(fn `Flamethrower Movement`
  (bind (_returnvalue_roll _returnvalue_pitch) (`KismetMathLibrary.BreakRotator` (`SceneComponent.K2_GetComponentRotation` (`self.ProjectileSpawnPoint`))))
  (bind (_returnvalue_roll_2 _returnvalue_pitch_2 _returnvalue_yaw) (`KismetMathLibrary.BreakRotator` (`KismetMathLibrary.Conv_VectorToRotator` (`self.GetActorForwardVector`))))
  (`self.SetProjectileSpwanPointRotation`)
  (`self.Server Update Ability transform` (`KismetMathLibrary.MakeTransform` (+ (* (`SceneComponent.GetForwardVector` (`self.CameraComponent`)) 100.0) (`self.K2_GetActorLocation`)) (`KismetMathLibrary.MakeRotator` _returnvalue_roll_2 _returnvalue_pitch _returnvalue_yaw)) (`KismetSystemLibrary.GetDisplayName` (`Controller.K2_GetPawn` (`GameplayStatics.GetPlayerController` 0))) (`KismetSystemLibrary.IsServer`) true))

(fn `GetVisorTransfrom`
  (returns (`Visor Transform` :type "Transform Structure"))
  (return (`KismetMathLibrary.MakeTransform` (+ (* (`SceneComponent.GetForwardVector` (`self.CameraComponent`)) 100.0) (`self.K2_GetActorLocation`)) (`SceneComponent.K2_GetComponentRotation` (`self.ProjectileSpawnPoint`)))))

(fn `IceThrower Movement`
  (bind (_returnvalue_roll _returnvalue_pitch) (`KismetMathLibrary.BreakRotator` (`SceneComponent.K2_GetComponentRotation` (`self.ProjectileSpawnPoint`))))
  (bind (_returnvalue_roll_2 _returnvalue_pitch_2 _returnvalue_yaw) (`KismetMathLibrary.BreakRotator` (`KismetMathLibrary.Conv_VectorToRotator` (`self.GetActorForwardVector`))))
  (`self.SetProjectileSpwanPointRotation`)
  (`self.Server Update Ability transform` (`KismetMathLibrary.MakeTransform` (+ (* (`SceneComponent.GetForwardVector` (`self.CameraComponent`)) 100.0) (`self.K2_GetActorLocation`)) (`KismetMathLibrary.MakeRotator` _returnvalue_roll_2 _returnvalue_pitch _returnvalue_yaw)) (`KismetSystemLibrary.GetDisplayName` (`Controller.K2_GetPawn` (`GameplayStatics.GetPlayerController` 0))) (`KismetSystemLibrary.IsServer`) true))

(fn `Meteor Movement`
  (params (`Ability Ref` :type "Actor Object Reference"))
  (bind _cameracomponent (`self.CameraComponent`))
  (bind _returnvalue (`SceneComponent.K2_GetComponentLocation` _cameracomponent))
  (`self.ZoomOutCameraView`)
  (`/Engine/EditorBlueprintResources/StandardMacros.IsValid` `Ability Ref`
    (:`Is Valid`
      (`self.SetProjectileSpwanPointRotation`)
      (bind (_outhit _returnvalue_2) (`KismetSystemLibrary.LineTraceSingle` _returnvalue (+ (* (`SceneComponent.GetForwardVector` _cameracomponent) 3000.0) _returnvalue) "TraceTypeQuery1"))
      (if _returnvalue_2
        (bind _output_get (set `self.Spawn Transform` (`KismetMathLibrary.MakeTransform` (`.Location` (`GameplayStatics.BreakHitResult` _outhit)) (`SceneComponent.K2_GetComponentRotation` (`self.ProjectileSpawnPoint`)))))
        (`self.K2_SetActorTransform` `Ability Ref` _output_get false false)))))

(fn `Second Ability Spawn`)

(fn `Second Ability Trigger Damage`
  (params (`Ability Ref` :type "Actor Object Reference"))
  (bind _asbp_elemental_game_instance (cast `/Game/Blueprints/BP_ElementalGameInstance` (`GameplayStatics.GetGameInstance`)))
  (switch `string` (`KismetSystemLibrary.GetClassDisplayName` (`/Game/Blueprints/BP_ElementalGameInstance.SecondAbilityClass` _asbp_elemental_game_instance))
    (:`BP_WaterDropletsAbility_C`
      (bind _asbp_water_droplets_ability (cast `/Game/Blueprints/Abilities/BP_WaterDropletsAbility` `Ability Ref`))
      (`/Game/Blueprints/Abilities/BP_WaterDropletsAbility.Trigger Damage` _asbp_water_droplets_ability))
    (:`BP_MeteorAbility_C`
      (bind _asbp_meteor_ability (cast `/Game/Blueprints/Abilities/BP_MeteorAbility` `Ability Ref`))
      (`/Game/Blueprints/Abilities/BP_MeteorAbility.TriggerDamage` _asbp_meteor_ability))
    (:`BP_TsunamiAbility_C`
      (bind _asbp_tsunami_ability (cast `/Game/Blueprints/Abilities/BP_TsunamiAbility` `Ability Ref`))
      (`/Game/Blueprints/Abilities/BP_TsunamiAbility.Trigger Damage` _asbp_tsunami_ability))
    (:`BP_BlizzardAbility_C`
      (bind _asbp_blizzard_ability (cast `/Game/Blueprints/Abilities/BP_BlizzardAbility` `Ability Ref`))
      (`/Game/Blueprints/Abilities/BP_BlizzardAbility.Trigger Damage` _asbp_blizzard_ability))))

(fn `SecondAbilitySpawnOnClick`
  (bind _secondabilityref (`self.SecondAbilityRef`))
  (bind (_returnvalue_location _returnvalue_rotation) (`KismetMathLibrary.BreakTransform` (`self.GetTransform` _secondabilityref)))
  (bind _asbp_elemental_game_instance (cast `/Game/Blueprints/BP_ElementalGameInstance` (`GameplayStatics.GetGameInstance`)))
  (bind _issecondabilityautospawn (`/Game/Blueprints/BP_ElementalGameInstance.IsSecondAbilityAutoSpawn` _asbp_elemental_game_instance))
  (if (not _issecondabilityautospawn)
    (bind _output_get (set `self.SecondAbilityTransform` (`KismetMathLibrary.MakeTransform` _returnvalue_location _returnvalue_rotation)))
    (`self.K2_DestroyActor` _secondabilityref)
    (set `self.FollowSecondAbility` false)
    (set `self.CanFireProjectile` true)
    (set `self.IsAlreadyInCast` false)
    (set `self.IsFirstAbilityCast` false)
    (`self.Server Spawn Second Ability` (`/Game/Blueprints/BP_ElementalGameInstance.SecondAbilityClass` _asbp_elemental_game_instance) _output_get _issecondabilityautospawn (`KismetSystemLibrary.IsServer`) (`self.IsAlreadyInCast`) (`Controller.K2_GetPawn` (`GameplayStatics.GetPlayerController` 0)))
    (`self.ZoomInCameraView`)))

(fn `ServerAbilityUpdateMovements`
  (params (Transform :type "Transform Structure") (ClientName :type String) (IsServer :type Boolean) (IsFirstAbility :type Boolean))
  (locals (CharacterName :type String))
  (bind (_lefts _rights) (`KismetStringLibrary.Split` ClientName "r" "IgnoreCase" "FromEnd"))
  (bind _charactername (`local.CharacterName`))
  (bind _charactername_2 (`local.CharacterName`))
  (if IsServer
    (set `local.CharacterName` ClientName)
    (else
      (set `local.CharacterName` (`KismetStringLibrary.Concat_StrStr` (`KismetStringLibrary.Concat_StrStr` _lefts "r_C_") _rights))))
  (bind _asbp_elemental_defender_game_mode_base (cast `/Game/Blueprints/BP_ElementalDefenderGameModeBase` (`GameplayStatics.GetGameMode`)))
  (if IsFirstAbility
    (if (`KismetArrayLibrary.Array_Contains` (`/Game/Blueprints/BP_ElementalDefenderGameModeBase.ServerFirstAbilityClientList` _asbp_elemental_defender_game_mode_base) _charactername_2)
      (`self.K2_SetActorTransform` (`|GetArrayItem` (`/Game/Blueprints/BP_ElementalDefenderGameModeBase.ServerAbilityRefList` _asbp_elemental_defender_game_mode_base) (`KismetArrayLibrary.Array_Find` (`/Game/Blueprints/BP_ElementalDefenderGameModeBase.ServerFirstAbilityClientList` _asbp_elemental_defender_game_mode_base) _charactername_2)) Transform false false))
    (elif (`KismetArrayLibrary.Array_Contains` (`/Game/Blueprints/BP_ElementalDefenderGameModeBase.ServerSecondAbilityClientLists` _asbp_elemental_defender_game_mode_base) _charactername)
      (`self.K2_SetActorTransform` (`|GetArrayItem` (`/Game/Blueprints/BP_ElementalDefenderGameModeBase.ServerAbilityRefList` _asbp_elemental_defender_game_mode_base) (`KismetArrayLibrary.Array_Find` (`/Game/Blueprints/BP_ElementalDefenderGameModeBase.ServerSecondAbilityClientLists` _asbp_elemental_defender_game_mode_base) _charactername)) Transform false false))))

(fn `TsunamiAbilityMovement`
  (params (`Ability Ref` :type "Actor Object Reference"))
  (bind _cameracomponent (`self.CameraComponent`))
  (bind _returnvalue (`SceneComponent.K2_GetComponentRotation` (`self.ProjectileSpawnPoint`)))
  (bind _returnvalue_2 (`SceneComponent.K2_GetComponentLocation` _cameracomponent))
  (`self.ZoomOutCameraView`)
  (`/Engine/EditorBlueprintResources/StandardMacros.IsValid` `Ability Ref`
    (:`Is Valid`
      (`self.SetProjectileSpwanPointRotation`)
      (bind (_outhit _returnvalue_3) (`KismetSystemLibrary.LineTraceSingle` _returnvalue_2 (+ (* (`SceneComponent.GetForwardVector` _cameracomponent) 3000.0) _returnvalue_2) "TraceTypeQuery1"))
      (if _returnvalue_3
        (bind (_bblockinghit _binitialoverlap _time _distance _location) (`GameplayStatics.BreakHitResult` _outhit))
        (set `self.Spawn Transform` (`KismetMathLibrary.MakeTransform` _location _returnvalue))
        (`self.K2_SetActorTransform` `Ability Ref` (`KismetMathLibrary.MakeTransform` _location _returnvalue (25.0 15.0 1.0)) false false)))))

(fn `UserConstructionScript`)

(fn `Water Droplets Movement`
  (params (`Ability Ref` :type "Actor Object Reference"))
  (bind _cameracomponent (`self.CameraComponent`))
  (bind _returnvalue (`SceneComponent.K2_GetComponentLocation` _cameracomponent))
  (`self.ZoomOutCameraView`)
  (`/Engine/EditorBlueprintResources/StandardMacros.IsValid` `Ability Ref`
    (:`Is Valid`
      (`self.SetProjectileSpwanPointRotation`)
      (bind (_outhit _returnvalue_2) (`KismetSystemLibrary.LineTraceSingle` _returnvalue (+ (* (`SceneComponent.GetForwardVector` _cameracomponent) 3000.0) _returnvalue) "TraceTypeQuery1"))
      (if _returnvalue_2
        (bind _output_get (set `self.Spawn Transform` (`KismetMathLibrary.MakeTransform` (`.Location` (`GameplayStatics.BreakHitResult` _outhit)) (`SceneComponent.K2_GetComponentRotation` (`self.ProjectileSpawnPoint`)))))
        (`self.K2_SetActorTransform` `Ability Ref` _output_get false false)))))

(fn `ZoomInCameraView`
  (set `SpringArmComponent.TargetArmLength` 600.0 (`self.CameraSpringArm`)))

(fn `ZoomOutCameraView`
  (set `SpringArmComponent.TargetArmLength` 1500.0 (`self.CameraSpringArm`)))