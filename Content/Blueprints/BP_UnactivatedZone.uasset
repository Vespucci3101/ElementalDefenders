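; Interactable zone actor that an elemental character activates to start a progress countup, with a damage-driven health bar.
; Capsule overlap gives BP_ElementalCharacter a reference to the zone and shows prompts, unless activated or reset.
; TriggerZone swaps the sphere material, fires lightning Niagara, starts the Progress component and reveals its percentage widget.
; Tick refreshes progress and turns widgets toward the camera; AnyDamage lowers a separately tracked UIHealth for the bar.
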(event `Update Progress`
  (bind _aswbp_progress (cast `/Game/UI/WBP_Progress` (`WidgetComponent.GetWidget` (`self.ProgressWidget`))))
  (`TextBlock.SetText` (`/Game/UI/WBP_Progress.ProgressText` _aswbp_progress) (`KismetTextLibrary.Conv_StringToText` (`KismetStringLibrary.Concat_StrStr` (`KismetStringLibrary.Conv_Int64ToString` (`KismetMathLibrary.FTrunc64` (`ProgressComponent.currentProgress` (`self.Progress`)))) "%"))))

(event `Trigger Zone`
  (set `self.IsActivated` true)
  (`PrimitiveComponent.SetMaterial` (`self.ZoneDimensionSphere`) 0 "/Engine/VREditor/UI/DiscMaterial.DiscMaterial")
  (`ActorComponent.SetActive` (`self.NS_Lightning`) true true)
  (`SceneComponent.SetVisibility` (`self.Interact1`) false false)
  (`SceneComponent.SetVisibility` (`self.Interact`) false false)
  (`ProgressComponent.StartProgress` (`self.Progress`))
  (`SceneComponent.SetVisibility` (`self.ProgressWidget`) true false))

(event `OnComponentBeginOverlap_Event`
  (params (OverlappedComponent :type "PrimitiveComponent Object Reference") (OtherActor :type "Actor Object Reference") (OtherComp :type "PrimitiveComponent Object Reference") (OtherBodyIndex :type Integer) (bFromSweep :type Boolean) (SweepResult :type "HitResult Structure (by ref)"))
  (if (and (not (`self.IsActivated`)) (not (`self.IsReset`)))
    (bind _asbp_elemental_character (cast `/Game/Blueprints/BP_ElementalCharacter` OtherActor))
    (set `/Game/Blueprints/BP_ElementalCharacter.CanInteractWithZone` true _asbp_elemental_character)
    (set `/Game/Blueprints/BP_ElementalCharacter.InteractableZone` self _asbp_elemental_character)
    (`SceneComponent.SetVisibility` (`self.Interact1`) true false)
    (`SceneComponent.SetVisibility` (`self.Interact`) true false)))

(event `OnComponentEndOverlap_Event`
  (params (OverlappedComponent :type "PrimitiveComponent Object Reference") (OtherActor :type "Actor Object Reference") (OtherComp :type "PrimitiveComponent Object Reference") (OtherBodyIndex :type Integer))
  (bind _asbp_elemental_character (cast `/Game/Blueprints/BP_ElementalCharacter` OtherActor))
  (set `/Game/Blueprints/BP_ElementalCharacter.CanInteractWithZone` false _asbp_elemental_character)
  (`SceneComponent.SetVisibility` (`self.Interact1`) false false)
  (`SceneComponent.SetVisibility` (`self.Interact`) false false))

(event `self.ReceiveBeginPlay`
  (bind _capsule (`self.Capsule`))
  (set `self.UIHealth` (`HealthComponent.maxHealth` (`self.Health`)))
  (`self.Server Update Health Bar` 0.0)
  (add `PrimitiveComponent.OnComponentBeginOverlap` _capsule (delegate `OnComponentBeginOverlap_Event`))
  (add `PrimitiveComponent.OnComponentEndOverlap` _capsule (delegate `OnComponentEndOverlap_Event`))
  (`SceneComponent.SetVisibility` (`self.Interact1`) false false)
  (`SceneComponent.SetVisibility` (`self.Interact`) false false)
  (`SceneComponent.SetVisibility` (`self.ProgressWidget`) false false))

(event `self.ReceiveTick`
  (params (DeltaSeconds :type "Float (single-precision)"))
  (bind _healthbar (`self.HealthBar`))
  (bind _returnvalue (`KismetMathLibrary.FindLookAtRotation` (`SceneComponent.K2_GetComponentLocation` _healthbar) (`SceneComponent.K2_GetComponentLocation` (`PlayerCameraManager.TransformComponent` (`GameplayStatics.GetPlayerCameraManager` 0)))))
  (`SceneComponent.K2_SetWorldRotation` _healthbar _returnvalue false false)
  (`SceneComponent.K2_SetWorldRotation` (`self.Interact1`) _returnvalue false false)
  (`SceneComponent.K2_SetWorldRotation` (`self.Interact`) _returnvalue false false)
  (if (`self.IsActivated`)
    (`self.Update Progress`)
    (`SceneComponent.K2_SetWorldRotation` (`self.ProgressWidget`) _returnvalue false false)
    (else
      (`SceneComponent.SetVisibility` (`self.ProgressWidget`) false false))))

(event `Server Update Health Bar`
  (params (DamageTaken :type "Float (double-precision)"))
  (bind _returnvalue (- (`self.UIHealth`) DamageTaken))
  (bind _aswbp_health_bar (cast `/Game/UI/WBP_HealthBar` (`WidgetComponent.GetWidget` (`self.HealthBar`))))
  (`ProgressBar.SetPercent` (`/Game/UI/WBP_HealthBar.HealthBar` _aswbp_health_bar) (/ _returnvalue (`HealthComponent.maxHealth` (`self.Health`))))
  (set `self.UIHealth` _returnvalue))

(event `self.ReceiveAnyDamage`
  (params (Damage :type "Float (single-precision)") (DamageType :type "DamageType Object Reference") (InstigatedBy :type "Controller Object Reference") (DamageCauser :type "Actor Object Reference"))
  (`self.Server Update Health Bar` Damage))

(fn `UserConstructionScript`)