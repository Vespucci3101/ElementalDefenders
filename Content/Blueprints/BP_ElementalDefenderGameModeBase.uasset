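; BP_ElementalDefenderGameModeBase is the game mode that tracks connected players and spawns their elemental characters.
; Login, logout and controller-swap events maintain the AllPcs list.
; Login and logout also tell BP_ElementalGameState, after a half-second delay, to refresh its player list.
; SpawnPlayer destroys any existing pawn, spawns a BP_ElementalCharacter at a random PlayerStart and possesses it with the given controller.
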(event `self.ReceiveBeginPlay`)

(event `UpdatePlayerLists`
  (`KismetSystemLibrary.Delay` 0.5)
  (bind _asbp_elemental_game_state (cast `/Game/Blueprints/BP_ElementalGameState` (`GameplayStatics.GetGameState`)))
  (`/Game/Blueprints/BP_ElementalGameState.Update Player List` _asbp_elemental_game_state))

(event `self.K2_PostLogin`
  (params (NewPlayer :type "PlayerController Object Reference"))
  (`KismetArrayLibrary.Array_Add` (`self.All Pcs`) NewPlayer)
  (`self.UpdatePlayerLists` :!label _label))

(event `self.K2_OnLogout`
  (params (ExitingController :type "Controller Object Reference"))
  (bind _asbp_elemental_player_controller (cast `/Game/Blueprints/BP_elementalPlayerController` ExitingController))
  (`KismetArrayLibrary.Array_RemoveItem` (`self.All Pcs`) _asbp_elemental_player_controller)
  (goto _label))

(event `self.K2_OnSwapPlayerControllers`
  (params (OldPC :type "PlayerController Object Reference") (NewPC :type "PlayerController Object Reference"))
  (`KismetArrayLibrary.Array_Add` (`self.All Pcs`) NewPC))

(fn `FindRandomPlayerStart`
  (returns (ReturnValue :type "Transform Structure (by ref)"))
  (bind _outactors (`GameplayStatics.GetAllActorsOfClass` "/Script/Engine.PlayerStart"))
  (return (`self.GetTransform` (`|GetArrayItem` _outactors (`KismetMathLibrary.RandomIntegerInRange` 0 (- (`KismetArrayLibrary.Array_Length` _outactors) 1))))))

(fn `SpawnPlayer`
  (params (PlayerController :type "PlayerController Object Reference"))
  (bind _returnvalue (`Controller.K2_GetPawn` PlayerController))
  (`/Engine/EditorBlueprintResources/StandardMacros.IsValid` _returnvalue
    (:`Is Valid`
      (`self.K2_DestroyActor` _returnvalue))
    (:`Is Not Valid`
      _))
  (bind _returnvalue_2 (`|SpawnActorFromClass` "/Game/Blueprints/BP_ElementalCharacter.BP_ElementalCharacter_C" (`self.FindRandomPlayerStart`) "Undefined" "OverrideRootScale" null null))
  (`Controller.Possess` PlayerController _returnvalue_2))

(fn `UserConstructionScript`)