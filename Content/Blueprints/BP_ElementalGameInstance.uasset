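; Game instance that holds the player's elemental class (Fire, Water or Ice) and the ability classes that go with it.
; One event stores the chosen class, and two others switch on it to set the first and second ability actor classes with their auto-spawn flags.
; The stored class change does not refresh the abilities itself, as each update is a separate event.
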(event `ChangePlayerClass`
  (params (CharacterClass :type String))
  (set `self.CharacterClass` CharacterClass))

(event `ChangeFirstAbilityActor`
  (switch `string` (`self.CharacterClass`)
    (:`Fire`
      (set `self.FirstAbilityClass` "/Game/Blueprints/Abilities/BP_FlameThrowerAbility.BP_FlameThrowerAbility_C")
      (set `self.IsFirstAbilityAutoSpawn` true))
    (:`Water`
      (set `self.FirstAbilityClass` "/Game/Blueprints/Abilities/BP_WaterDropletsAbility.BP_WaterDropletsAbility_C")
      (set `self.IsFirstAbilityAutoSpawn` false))
    (:`Ice`
      (set `self.FirstAbilityClass` "/Game/Blueprints/Abilities/BP_IceThrowerAbility.BP_IceThrowerAbility_C")
      (set `self.IsFirstAbilityAutoSpawn` true))))

(event `ChangeSecondAbilityActor`
  (switch `string` (`self.CharacterClass`)
    (:`Fire`
      (set `self.SecondAbilityClass` "/Game/Blueprints/Abilities/BP_MeteorAbility.BP_MeteorAbility_C")
      (set `self.IsSecondAbilityAutoSpawn` false))
    (:`Water`
      (set `self.SecondAbilityClass` "/Game/Blueprints/Abilities/BP_TsunamiAbility.BP_TsunamiAbility_C")
      (set `self.IsSecondAbilityAutoSpawn` false))
    (:`Ice`
      (set `self.SecondAbilityClass` "/Game/Blueprints/Abilities/BP_BlizzardAbility.BP_BlizzardAbility_C")
      (set `self.IsSecondAbilityAutoSpawn` false))))