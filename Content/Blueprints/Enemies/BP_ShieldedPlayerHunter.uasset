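; Shielded player-hunter enemy Blueprint; this graph handles only its floating health bar.
; Each tick the HealthBar widget component rotates to face the first player's camera.
; AnyDamage feeds ServerUpdateHealth, which subtracts damage from a separate UIHealth copy, seeded from the Health component's MaxHealth, and sets the WBP_HealthBar percentage.
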(event `self.ReceiveBeginPlay`
  (set `self.UIHealth` (`HealthComponent.maxHealth` (`self.Health`)))
  (`self.Server Update Health` 0.0))

(event `self.ReceiveTick`
  (params (DeltaSeconds :type "Float (single-precision)"))
  (bind _healthbar (`self.HealthBar`))
  (`SceneComponent.K2_SetWorldRotation` _healthbar (`KismetMathLibrary.FindLookAtRotation` (`SceneComponent.K2_GetComponentLocation` _healthbar) (`SceneComponent.K2_GetComponentLocation` (`PlayerCameraManager.TransformComponent` (`GameplayStatics.GetPlayerCameraManager` 0)))) false false))

(event `Server Update Health`
  (params (`Damage Taken` :type "Float (double-precision)"))
  (bind _returnvalue (- (`self.UIHealth`) `Damage Taken`))
  (bind _aswbp_health_bar (cast `/Game/UI/WBP_HealthBar` (`WidgetComponent.GetWidget` (`self.HealthBar`))))
  (`ProgressBar.SetPercent` (`/Game/UI/WBP_HealthBar.HealthBar` _aswbp_health_bar) (/ _returnvalue (`HealthComponent.maxHealth` (`self.Health`))))
  (set `self.UIHealth` _returnvalue))

(event `self.ReceiveAnyDamage`
  (params (Damage :type "Float (single-precision)") (DamageType :type "DamageType Object Reference") (InstigatedBy :type "Controller Object Reference") (DamageCauser :type "Actor Object Reference"))
  (`self.Server Update Health` Damage))

(fn `UserConstructionScript`)