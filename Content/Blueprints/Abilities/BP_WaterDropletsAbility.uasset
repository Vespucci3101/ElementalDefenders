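; BP_WaterDropletsAbility is the water droplets ability actor, treated as an elemental character's first ability.
; TriggerDamage sets the damage flag and timestamps a time-to-live, which Tick polls to clear the flag and destroy the actor.
; CancelAbility destroys it immediately.
; On destruction it restores the owning character's cast and projectile state and removes itself from the game mode's element lists.
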(event `self.ReceiveBeginPlay`
  (set `self.StartTime` -1.0))

(event `self.ReceiveTick`
  (params (DeltaSeconds :type "Float (single-precision)"))
  (bind _starttime (`self.StartTime`))
  (if (and (!= _starttime -1.0) (>= (- (`GameplayStatics.GetTimeSeconds`) _starttime) (`self.TTL`)))
    (set `self.isDamageTriggered` false)
    (`self.K2_DestroyActor`)))

(event `Cancel Ability`
  (`self.K2_DestroyActor`))

(event `Trigger Damage`
  (`self.TriggerTimeToLive`)
  (set `self.isDamageTriggered` true))

(event `TriggerTimeToLive`
  (set `self.StartTime` (`GameplayStatics.GetTimeSeconds`)))

(event `self.ReceiveDestroyed`
  (bind _returnvalue (`self.GetOwner`))
  (bind _asbp_elemental_character (cast `/Game/Blueprints/BP_ElementalCharacter` _returnvalue))
  (set `/Game/Blueprints/BP_ElementalCharacter.CanFireProjectile` true _asbp_elemental_character)
  (set `/Game/Blueprints/BP_ElementalCharacter.IsAlreadyInCast` false _asbp_elemental_character)
  (set `/Game/Blueprints/BP_ElementalCharacter.FollowFirstAbility` false _asbp_elemental_character)
  (bind _asbp_elemental_defender_game_mode_base (cast `/Game/Blueprints/BP_ElementalDefenderGameModeBase` (`GameplayStatics.GetGameMode`)))
  (`/Game/Blueprints/BP_ElementalDefenderGameModeBase.RemoveElementFromLists` _asbp_elemental_defender_game_mode_base self true (`KismetSystemLibrary.GetDisplayName` _returnvalue)))

(fn `UserConstructionScript`)