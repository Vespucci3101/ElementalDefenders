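; BP_Projectile is an ability projectile whose look reflects an elemental character class.
; Its SetProjectileClass event switches on the given class (Fire, Water, Earth, Herb, Ice, Air or Void) and applies that element's materials to the projectile mesh and its wisp.
; The graphs hold no movement, collision or damage logic; BeginPlay, overlap, Tick and the construction script are empty.
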(event `self.ReceiveBeginPlay`)

(event `Set Projectile Class`
  (params (`Character Class` :type String))
  (switch `string` `Character Class`
    (:`Fire`
      (`PrimitiveComponent.SetMaterial` (`self.projectileMesh`) 0 "/Game/Materials/Fire/M_ProjectileFire.M_ProjectileFire")
      (`PrimitiveComponent.SetMaterial` (`self.Wisp`) 0 "/Game/Materials/Fire/M_WispFire.M_WispFire"))
    (:`Water`
      (`PrimitiveComponent.SetMaterial` (`self.projectileMesh`) 0 "/Game/Materials/Water/M_ProjectileWater.M_ProjectileWater")
      (`PrimitiveComponent.SetMaterial` (`self.Wisp`) 0 "/Game/Materials/Water/M_WispWater.M_WispWater"))
    (:`Earth`
      (`PrimitiveComponent.SetMaterial` (`self.projectileMesh`) 0 "/Game/Materials/Earth/M_ProjectileEarth.M_ProjectileEarth")
      (`PrimitiveComponent.SetMaterial` (`self.Wisp`) 0 "/Game/Materials/Earth/M_WispEarth.M_WispEarth"))
    (:`Herb`
      (`PrimitiveComponent.SetMaterial` (`self.projectileMesh`) 0 "/Game/Materials/Herb/M_ProjectileHerb.M_ProjectileHerb")
      (`PrimitiveComponent.SetMaterial` (`self.Wisp`) 0 "/Game/Materials/Herb/M_WispHerb.M_WispHerb"))
    (:`Ice`
      (`PrimitiveComponent.SetMaterial` (`self.projectileMesh`) 0 "/Game/Materials/Ice/M_ProjectileIce.M_ProjectileIce")
      (`PrimitiveComponent.SetMaterial` (`self.Wisp`) 0 "/Game/Materials/Ice/M_WispIce.M_WispIce"))
    (:`Air`
      (`PrimitiveComponent.SetMaterial` (`self.projectileMesh`) 0 "/Game/Materials/Air/M_ProjectileAir.M_ProjectileAir")
      (`PrimitiveComponent.SetMaterial` (`self.Wisp`) 0 "/Game/Materials/Air/M_WispAir.M_WispAir"))
    (:`Void`
      (`PrimitiveComponent.SetMaterial` (`self.projectileMesh`) 0 "/Game/Materials/Void/M_ProjectileVoid.M_ProjectileVoid")
      (`PrimitiveComponent.SetMaterial` (`self.Wisp`) 0 "/Game/Materials/Void/M_WispVoid.M_WispVoid"))))

(fn `UserConstructionScript`)