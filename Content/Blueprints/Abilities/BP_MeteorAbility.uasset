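; BP_MeteorAbility is a second-slot ability actor that drops a meteor on its MeteorMesh location.
; TriggerDamage spawns BP_Meteor high above the mesh with a straight-down, gravity-free velocity.
; Tick detects the meteor reaching world Z zero, spawns an explosion, calls DealDamage and destroys the ability after a short delay.
; Destruction, including cancellation, resets the owning character's casting flags and removes the ability from GameMode lists.
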(event `self.ReceiveBeginPlay`)

(event `self.ReceiveTick`
  (params (DeltaSeconds :type "Float (single-precision)"))
  (bind _meteorref (`self.MeteorRef`))
  (bind _meteormesh (`self.MeteorMesh`))
  (bind (_returnvalue_x _returnvalue_y _returnvalue_z) (`KismetMathLibrary.BreakVector` (`self.K2_GetActorLocation` _meteorref)))
  (if (not (`self.IsMeteorDestroyed`))
    (`/Engine/EditorBlueprintResources/StandardMacros.IsValid` _meteorref
      (:`Is Valid`
        (if (<= _returnvalue_z 0.0)
          (bind _returnvalue (`|SpawnActorFromClass` "/Game/Blueprints/Effects/BP_Explosion.BP_Explosion_C" (`KismetMathLibrary.MakeTransform` (+ (`SceneComponent.K2_GetComponentLocation` _meteormesh) (0.0 0.0 25.0)) (`SceneComponent.K2_GetComponentRotation` _meteormesh)) "Undefined" "OverrideRootScale" null null))
          (`ActorComponent.SetActive` (`/Game/Blueprints/Effects/BP_Explosion.Niagara` _returnvalue) true true)
          (`self.K2_DestroyActor` (`self.MeteorRef`))
          (set `self.IsMeteorDestroyed` true)
          (`self.DealDamage`)
          (`KismetSystemLibrary.Delay` 1.0)
          (`self.K2_DestroyActor`))))))

(event `self.ReceiveDestroyed`
  (bind _returnvalue (`self.GetOwner`))
  (bind _asbp_elemental_character (cast `/Game/Blueprints/BP_ElementalCharacter` _returnvalue))
  (set `/Game/Blueprints/BP_ElementalCharacter.CanFireProjectile` true _asbp_elemental_character)
  (set `/Game/Blueprints/BP_ElementalCharacter.IsAlreadyInCast` false _asbp_elemental_character)
  (set `/Game/Blueprints/BP_ElementalCharacter.FollowSecondAbility` false _asbp_elemental_character)
  (bind _asbp_elemental_defender_game_mode_base (cast `/Game/Blueprints/BP_ElementalDefenderGameModeBase` (`GameplayStatics.GetGameMode`)))
  (`/Game/Blueprints/BP_ElementalDefenderGameModeBase.RemoveElementFromLists` _asbp_elemental_defender_game_mode_base self false (`KismetSystemLibrary.GetDisplayName` _returnvalue)))

(event `TriggerDamage`
  (bind _meteormesh (`self.MeteorMesh`))
  (bind _returnvalue (`|SpawnActorFromClass` "/Game/Blueprints/Effects/BP_Meteor.BP_Meteor_C" (`KismetMathLibrary.MakeTransform` (+ (`SceneComponent.K2_GetComponentLocation` _meteormesh) (0.0 0.0 3000.0)) (`SceneComponent.K2_GetComponentRotation` _meteormesh)) "Undefined" "OverrideRootScale" null null))
  (`ActorComponent.SetActive` (`/Game/Blueprints/Effects/BP_Meteor.Niagara` _returnvalue) true true)
  (bind _projectilemovement (`/Game/Blueprints/Effects/BP_Meteor.ProjectileMovement` _returnvalue))
  (set `MovementComponent.Velocity` (0.0 0.0 -1500.0) _projectilemovement)
  (set `ProjectileMovementComponent.ProjectileGravityScale` 0.0 _projectilemovement)
  (set `self.MeteorRef` _returnvalue))

(event `Cancel Ability`
  (`self.K2_DestroyActor`))

(fn `UserConstructionScript`)